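; Rifle weapon actor that handles the automatic-fire cadence, with no projectile, trace or damage logic in this graph.
; BeginPlay sets the tick interval from RateOfFire, so each Tick acts as one shot.
; The Fire event toggles the Shooting flag.
; While it is set, Tick prints a debug string and calls WeaponForceFeedback on player 0's Ue4ASP_Character, regardless of who holds the weapon.
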(event `self.ReceiveBeginPlay`
  (`self.SetActorTickInterval` (/ 1.0 (`self.RateOfFire`))))

(event `self.ReceiveTick`
  (params (DeltaSeconds :type "Float (single-precision)"))
  (if (`self.Shooting`)
    (`KismetSystemLibrary.PrintString` "Weapon")
    (bind _asue_4asp_character (cast `/Game/Characters/X/Ue4ASP_Character` (`Controller.K2_GetPawn` (`GameplayStatics.GetPlayerController` 0))))
    (`/Game/Characters/X/Ue4ASP_Character.WeaponForceFeedback` _asue_4asp_character)))

(event `Fire`
  (params (Shoot :type Boolean))
  (set `self.Shooting` Shoot))

(fn `UserConstructionScript`)